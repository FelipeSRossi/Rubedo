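; ExaminedItemCapture is an actor that holds the item currently being examined, presumably for a capture view.
; On BeginPlay it stores itself in an ExaminedItemCapture reference and takes its ChildActor component's actor as the starting item.
; ChangeExaminedItem spawns the requested class at the StaticMesh's world transform, ignoring collisions, then destroys the previous item after a root-component check and tracks the new one.
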(event `self.ReceiveBeginPlay`
  (set `self.ExaminedItemCapture` self)
  (set `self.CurrentItem` (`ChildActorComponent.ChildActor` (`self.ChildActor`))))

(event `/Game/Blueprints/BPI_ExaminedItem.ChangeExaminedItem`
  (params (NewItem :type "Actor Class Reference"))
  (bind _currentitem (`self.CurrentItem`))
  (bind _returnvalue (`|SpawnActorFromClass` NewItem (`SceneComponent.K2_GetComponentToWorld` (`self.StaticMesh`)) "AlwaysSpawn" "OverrideRootScale" null null))
  (if (!= (`Actor.RootComponent` _currentitem) null)
    (`self.K2_DestroyActor` _currentitem))
  (set `self.CurrentItem` _returnvalue))

(fn `UserConstructionScript`)