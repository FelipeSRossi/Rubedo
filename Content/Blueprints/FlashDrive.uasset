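; FlashDrive is a pickup item that spins in the world and can be added to the player's inventory.
; Interact pauses the game and shows an ItemInteract Yes/No prompt with the item's name.
; Both buttons close it and restore game input; Yes also passes ItemInfoStruct to the PlayerCharacter's inventory widget and destroys the actor.
; UseItem only prints a debug string, and the Tick spin is frame-rate dependent.
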(event `/Game/InventorySystem/InteractInterface.Interact`
  (bind _item_interact_widget_ref (`self.Item Interact Widget REF`))
  (bind _yesbutton (`/Game/Menus/ItemInteract.YesButton` _item_interact_widget_ref))
  ;[1 1 1] Create Yes/No HUD
  (bind _returnvalue (`|CreateWidget` "/Game/Menus/ItemInteract.ItemInteract_C"))
  (set `self.Item Interact Widget REF` _returnvalue)
  (`EditableText.SetText` (`/Game/Menus/ItemInteract.EditableText_353` _item_interact_widget_ref) (`KismetTextLibrary.Conv_StringToText` (`KismetStringLibrary.Concat_StrStr` "Get " (`.Name_2_B07E00E6443FC1472370EE83B99C2380` (break `/Game/InventorySystem/Struct_ItemInfo` (`self.ItemInfoStruct`))) " ?")))
  (`UserWidget.AddToViewport` _item_interact_widget_ref 0)
  (`Widget.SetFocus` _yesbutton)
  (add `Button.OnPressed` (`/Game/Menus/ItemInteract.NoButton` _item_interact_widget_ref) (delegate `NoPressed`))
  (add `Button.OnPressed` _yesbutton (delegate `YesPressed`))
  (`GameplayStatics.SetGamePaused` true))

(event `NoPressed`
  ;[1 1 1] No Button
  (`Widget.RemoveFromParent` (`self.Item Interact Widget REF`))
  (`WidgetBlueprintLibrary.SetInputMode_GameOnly` (`GameplayStatics.GetPlayerController` 0))
  (`GameplayStatics.SetGamePaused` false))

(event `YesPressed`
  ;[1 1 1] Yes Button
  (`Widget.RemoveFromParent` (`self.Item Interact Widget REF`))
  (`WidgetBlueprintLibrary.SetInputMode_GameOnly` (`GameplayStatics.GetPlayerController` 0))
  (bind _asplayer_character (cast `/Game/CharacterBlueprints/PlayerCharacter` (`GameplayStatics.GetPlayerCharacter` 0)))
  (`GameplayStatics.SetGamePaused` false)
  (`/Game/InventorySystem/UI/InventoryWG.AddToInventory` (`/Game/CharacterBlueprints/PlayerCharacter.Inventory WDG` _asplayer_character) (`self.ItemInfoStruct`))
  (`self.K2_DestroyActor`))

(event `/Game/InventorySystem/InteractInterface.UseItem`
  (`KismetSystemLibrary.PrintString` "UseFlashDrive"))

(event `self.ReceiveTick`
  (params (DeltaSeconds :type "Float (single-precision)"))
  (`SceneComponent.K2_AddLocalRotation` (`self.DefaultSceneRoot`) (`KismetMathLibrary.MakeRotator` 0.0 0.0 (+ DeltaSeconds 1.0)) false false))

(fn `UserConstructionScript`
  (`parent.UserConstructionScript`))