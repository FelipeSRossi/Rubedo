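; CutsceneManager_BP is a Blueprint whose only active logic toggles a pause menu, despite its cutscene-manager name.
; PauseCall lazily creates and caches the menu widget in PauseMenuREF, then branches on whether the game is paused.
; It adds or removes the widget, sets the pause state, and switches cursor visibility and input mode between game-and-UI and game-only.
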(event `/Game/Blueprints/BPI_CutscenePlayer.Pause Call`
  (bind _returnvalue (`GameplayStatics.GetPlayerController` 0))
  (bind _pause_menu_ref (`self.Pause Menu REF`))
  ;[1 1 1] Pause/Unpause
  (`/Engine/EditorBlueprintResources/StandardMacros.IsValid` (`self.Pause Menu REF`)
    (:`Is Valid`
      _)
    (:`Is Not Valid`
      (bind _returnvalue_2 (`|CreateWidget` "/Game/Menus/PauseMenuWidget.PauseMenuWidget_C"))
      (set `self.Pause Menu REF` _returnvalue_2)))
  (if (`GameplayStatics.IsGamePaused`)
    (`Widget.RemoveFromParent` _pause_menu_ref)
    (`GameplayStatics.SetGamePaused` false)
    (set `PlayerController.bShowMouseCursor` false _returnvalue)
    (`WidgetBlueprintLibrary.SetInputMode_GameOnly` _returnvalue)
    (else
      (`UserWidget.AddToViewport` _pause_menu_ref 0)
      (`GameplayStatics.SetGamePaused` true)
      (set `PlayerController.bShowMouseCursor` true _returnvalue)
      (`WidgetBlueprintLibrary.SetInputMode_GameAndUIEx` _returnvalue _pause_menu_ref "LockInFullscreen"))))

(fn `UserConstructionScript`)